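; BP_GameObject is the base actor for interactable objects such as pickup items, random-item searches, backpacks and hiding spots.
; PickUpCollision overlaps enable input and gate the Interaction key, with a delayed shutoff for pickup items.
; Interaction switches on Type, either passing items to BP_Player or casting self to child Blueprints.
; It also provides dynamic-material color changes, timeline scale pulsing and float/rotate helpers, plus unconnected flicker logic.
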(event `IncreaseScale`
  (params (Duration :type "Float (double-precision)") (Scale :type "Float (double-precision)"))
  ;[1 1 1] Increase Scale
  (bind (_direction _scale) (`Timeline|TimelineBodyScale` :!via `PlayFromStart` :!label _label)
    (:`Update`
      (`SceneComponent.SetRelativeScale3D` (`self.DefaultSceneRoot`) (`KismetMathLibrary.Conv_DoubleToVector` (+ 1.0 (* _scale Scale)))))
    (:`Finished`
      (if (`self.ComponentScaledStatus`)
        (set `self.ComponentScaledStatus` false)
        (else
          (set `self.ComponentScaledStatus` true)
          (`KismetSystemLibrary.Delay` (- Duration (* (`TimelineComponent.GetTimelineLength` (`self.TimelineBodyScale`)) 2.0)))
          (goto _label :!via `ReverseFromEnd`))))))

(event `ChangeColorForDuration`
  (params (Duration :type "Float (double-precision)") (EyeColor :type "LinearColor Structure"))
  ;[1 1 1] Change Color
  (`MaterialInstanceDynamic.SetVectorParameterValue` (`self.VisualMeshMaterial`) "Color" EyeColor)
  (`KismetSystemLibrary.Delay` Duration)
  (`MaterialInstanceDynamic.SetVectorParameterValue` (`self.VisualMeshMaterial`) "Color" (`self.VisualMeshColor`)))

(event `ChangeColor`
  (params (EyeColor :type "LinearColor Structure"))
  ;[1 1 1] Change Color
  (`MaterialInstanceDynamic.SetVectorParameterValue` (`self.VisualMeshMaterial`) "Color" EyeColor))

(event `self.ReceiveBeginPlay`
  (bind _returnvalue (`PrimitiveComponent.CreateDynamicMaterialInstance` (`self.VisualMesh`) 0 null "None"))
  (bind _output_get (set `self.VisualMeshMaterial` _returnvalue))
  (bind _returnvalue_2 (`MaterialInstanceDynamic.K2_GetVectorParameterValue` _output_get "Color"))
  (set `self.VisualMeshColor` _returnvalue_2))

(event `self.ReceiveActorBeginOverlap`
  (params (OtherActor :type "Actor Object Reference")))

(event `self.ReceiveTick`
  (params (DeltaSeconds :type "Float (single-precision)")))

(event `InputAction|Interaction`
  (params (Key :type "Key Structure"))
  ;[1 1 1] Interaction with the GameObject
  (:`Pressed`
    (`/Engine/EditorBlueprintResources/StandardMacros.Gate` (`self.isClosed`) :!label _label_2
      (:`Exit`
        (switch `/Game/Code/TypeGameObject` (`self.type`)
          (:`NewEnumerator0`
            (`self.Search for Item`))
          (:`NewEnumerator2`
            (`self.Pick Up Back Pack`))
          (:`NewEnumerator6`
            (`self.Interact Hiding Spot`))
          (:`NewEnumerator7`
            (`self.PickUpItem` "/Game/Code/Items/BP_EnergyDrink.BP_EnergyDrink_C" (`self.size`)))
          (:`NewEnumerator8`
            (`self.PickUpItem` "/Game/Code/Items/BP_Ball.BP_Ball_C" (`self.size`)))
          (:`NewEnumerator9`
            (`self.PickUpItem` "/Game/Code/Items/BP_Laptop.BP_Laptop_C" (`self.size`)))
          (:`NewEnumerator10`
            (`self.PickUpItem` "/Game/Code/Items/BP_Phone.BP_Phone_C" (`self.size`)))
          (:`NewEnumerator11`
            (`self.PickUpItem` "/Game/Code/Items/BP_TV.BP_TV_C" (`self.size`)))
          (:`NewEnumerator12`
            (`self.PickUpItem` "/Game/Code/Items/BP_Lamp.BP_Lamp_C" (`self.size`))))))))

(event `self.Pick Up Collision.OnComponentBeginOverlap`
  (params (OverlappedComponent :type "PrimitiveComponent Object Reference") (OtherActor :type "Actor Object Reference") (OtherComp :type "PrimitiveComponent Object Reference") (OtherBodyIndex :type Integer) (bFromSweep :type Boolean) (SweepResult :type "HitResult Structure (by ref)"))
  ;[1 1 1] Interaction with the GameObject
  (`KismetSystemLibrary.PrintString` "open")
  (`self.EnableInput` (`GameplayStatics.GetPlayerController` 0))
  (bind _asbp_player (cast `/Game/Code/Characters/BP_Player` OtherActor))
  (if (`|EnumEquality` (`self.type`) "NewEnumerator0")
    (set `/Game/Code/Characters/BP_Player.showFkey` true _asbp_player)
    (goto _label_2 :!via `Open`)
    (else
      (goto _label_2 :!via `Open`))))

(event `self.Pick Up Collision.OnComponentEndOverlap`
  (params (OverlappedComponent :type "PrimitiveComponent Object Reference") (OtherActor :type "Actor Object Reference") (OtherComp :type "PrimitiveComponent Object Reference") (OtherBodyIndex :type Integer))
  ;[1 1 1] Interaction with the GameObject
  (switch `/Game/Code/TypeGameObject` (`self.type`)
    (:`NewEnumerator0`
      _)
    (:`NewEnumerator2`
      _)
    (:`NewEnumerator6`
      _)
    (:`NewEnumerator7`
      (`KismetSystemLibrary.Delay` 5.0 :!label _label_3))
    (:`NewEnumerator8`
      (goto _label_3))
    (:`NewEnumerator9`
      (goto _label_3))
    (:`NewEnumerator10`
      (goto _label_3))
    (:`NewEnumerator11`
      (goto _label_3))
    (:`NewEnumerator12`
      (goto _label_3)))
  (`self.DisableInput` (`GameplayStatics.GetPlayerController` 0))
  (bind _asbp_player (cast `/Game/Code/Characters/BP_Player` OtherActor))
  (if (`|EnumEquality` (`self.type`) "NewEnumerator0")
    (set `/Game/Code/Characters/BP_Player.showFkey` false _asbp_player)
    (bind _asbp_random_item (cast `/Game/Code/BP_RandomItem` self))
    (set `/Game/Code/BP_RandomItem.PickingUpItem` false _asbp_random_item)
    (goto _label_2 :!via `Close`)
    (else
      (goto _label_2 :!via `Close`))))

(fn `CheckRunningState`
  (returns (NewParam :type Boolean))
  ;[1 1 1] Check if running state is activated
  (bind _asbp_top_down_game_mode (cast `/Game/Base/BP_TopDownGameMode` (`GameplayStatics.GetGameMode`)))
  (bind _newparam (`/Game/Base/BP_TopDownGameMode.GetIsRunningState` _asbp_top_down_game_mode))
  (return _newparam))

(fn `floating`
  ;[1 1 1] Move the game object Up and Down repeatedly
  (`SceneComponent.K2_AddRelativeLocation` (`self.VisualMesh`) (`KismetMathLibrary.MakeVector` 0.0 0.0 (* (`KismetMathLibrary.Sin` (`self.GetGameTimeSinceCreation`)) 0.5)) false false))

(fn `GetPlayerInput`
  (params (actor :type "Actor Object Reference"))
  (returns (player :type "/Game/Code/Characters/BP_Player Object Reference"))
  (`self.EnableInput` (`GameplayStatics.GetPlayerController` 0))
  (bind _asbp_player (cast `/Game/Code/Characters/BP_Player` actor))
  (return _asbp_player))

(fn `Interact Hiding Spot`
  (bind _asbp_hiding_spot (cast `/Game/Code/BP_HidingSpot` self))
  (`/Game/Code/BP_HidingSpot.Use Hiding Spot` _asbp_hiding_spot))

(fn `IsFlickerTimeOver`
  (params (FlickerTimeTotal :type "Float (double-precision)"))
  (returns (ReturnValue :type Boolean))
  (bind _output_get (set `self.FlickerTime` (+ (`self.FlickerTime`) (`TimelineComponent.GetTimelineLength` (`self.Timeline_Flicker`)))))
  (return (>= _output_get FlickerTimeTotal)))

(fn `Pick Up Back Pack`
  (bind _asbp_backpack (cast `/Game/Code/Items/BP_Backpack` self))
  (`/Game/Code/Items/BP_Backpack.PickUpBackpack` _asbp_backpack)
  (`self.K2_DestroyActor` _asbp_backpack))

(fn `PickUpItem`
  (params (Item :type "/Game/Base/BP_GameObject Class Reference") (size :type Integer))
  (`KismetSystemLibrary.PrintString` (`KismetSystemLibrary.GetClassDisplayName` Item))
  (if (not (`self.isStolen`))
    (bind _asbp_player (cast `/Game/Code/Characters/BP_Player` (`GameplayStatics.GetPlayerCharacter` 0)))
    (bind _pickup (`/Game/Code/Characters/BP_Player.PickUpItem` _asbp_player Item size))
    (if _pickup
      (`self.K2_DestroyActor`)
      (else
        (set `/Game/Code/Characters/BP_Player.noSpaceLeft` true _asbp_player) ; For HUD animation
      ))))

(fn `rotate`
  (`SceneComponent.K2_AddRelativeRotation` (`self.VisualMesh`) (`KismetMathLibrary.MakeRotator` 0.0 0.0 (+ (`self.angleRotation`) 0.5)) false false))

(fn `Search for Item`
  (bind _asbp_random_item (cast `/Game/Code/BP_RandomItem` self))
  (bind _asbp_player (cast `/Game/Code/Characters/BP_Player` (`GameplayStatics.GetPlayerCharacter` 0)))
  (set `/Game/Code/Characters/BP_Player.firstShowed` false _asbp_player)
  (set `/Game/Code/BP_RandomItem.PickingUpItem` true _asbp_random_item))

(fn `setNrEnergyDrinks`)

(fn `UserConstructionScript`)