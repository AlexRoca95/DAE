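; Searchable box pickup that drops a random item when the player finishes searching it.
; Pick Up Item input, gated by player overlap, toggles searching, which bobs the mesh and fills a widget progress bar unless running; idle boxes float and rotate.
; On completion it makes a weighted roll, re-rolling types at their game-mode caps with no exit if all are full, spawns the item, increments its count and destroys itself.
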(event `self.ReceiveBeginPlay`
  (`parent.ReceiveBeginPlay`))

(event `self.ReceiveActorBeginOverlap`
  (params (OtherActor :type "Actor Object Reference"))
  (`parent.ReceiveActorBeginOverlap` OtherActor))

(event `self.ReceiveTick`
  (params (DeltaSeconds :type "Float (single-precision)"))
  (`parent.ReceiveTick` DeltaSeconds)
  (`|ExecutionSequence`
    (:`then_0`
      (`self.BoxAnimation`))
    (:`then_1`
      (bind _asbp_top_down_game_mode (cast `/Game/Base/BP_TopDownGameMode` (`GameplayStatics.GetGameMode`)))
      (bind _newparam (`/Game/Base/BP_TopDownGameMode.GetIsRunningState` _asbp_top_down_game_mode))
      (if (not _newparam)
        ;[1 1 1] Player searching for an Object in the box
        (`self.SearchForItem`)
        (`self.UpdateUIBar`)
        (`self.CheckProgressBar`)))
    (:`then_2`
      (`self.Hide/ShowBar`))))

(event `InputAction|Pick Up Item`
  (params (Key :type "Key Structure"))
  ;[1 1 1] Player Interaction with the box
  (:`Pressed`
    (`/Engine/EditorBlueprintResources/StandardMacros.Gate` true :!label _label
      (:`Exit`
        (if (`self.PickingUpItem`)
          (set `self.PickingUpItem` false)
          (else
            (set `self.PickingUpItem` true))))))
  (:`Released`
    (goto _label :!via `Close`)))

(event `self.PickUp Collision.OnComponentBeginOverlap`
  (params (OverlappedComponent :type "PrimitiveComponent Object Reference") (OtherActor :type "Actor Object Reference") (OtherComp :type "PrimitiveComponent Object Reference") (OtherBodyIndex :type Integer) (bFromSweep :type Boolean) (SweepResult :type "HitResult Structure (by ref)"))
  ;[1 1 1] Player Interaction with the box
  (`self.EnableInput` (`GameplayStatics.GetPlayerController` 0))
  (cast `/Game/Code/Characters/BP_Player` OtherActor)
  (goto _label :!via `Open`))

(event `self.PickUp Collision.OnComponentEndOverlap`
  (params (OverlappedComponent :type "PrimitiveComponent Object Reference") (OtherActor :type "Actor Object Reference") (OtherComp :type "PrimitiveComponent Object Reference") (OtherBodyIndex :type Integer))
  ;[1 1 1] Player Interaction with the box
  (`self.DisableInput` (`GameplayStatics.GetPlayerController` 0))
  (cast `/Game/Code/Characters/BP_Player` OtherActor)
  (set `self.PickingUpItem` false) ; Stop Animation when move
)

(fn `BoxAnimation`
  (if (`self.PickingUpItem`)
    (bind _newparam (`self.CheckRunningState`))
    (if (not _newparam)
      (`self.PickingUpAnimation`))
    (else
      (`|ExecutionSequence`
        (:`then_0`
          (`self.rotate`))
        (:`then_1`
          (`self.floating`))))))

(fn `Check Nr Balls`
  (returns (ReturnValue :type Boolean))
  (bind _newparam (`self.GetTopDownGame`))
  (return (< (`/Game/Base/BP_TopDownGameMode.nrBalls` _newparam) (`/Game/Base/BP_TopDownGameMode.maxBalls` _newparam))))

(fn `Check Nr Energy Drinks`
  (returns (ReturnValue :type Boolean))
  (bind _newparam (`self.GetTopDownGame`))
  (return (< (`/Game/Base/BP_TopDownGameMode.NrEnergyDrinks` _newparam) (`/Game/Base/BP_TopDownGameMode.maxEnergyDrinks` _newparam))))

(fn `Check Nr Lamps`
  (returns (ReturnValue :type Boolean))
  (bind _newparam (`self.GetTopDownGame`))
  (return (< (`/Game/Base/BP_TopDownGameMode.nrLamps` _newparam) (`/Game/Base/BP_TopDownGameMode.maxLamps` _newparam))))

(fn `Check Nr Laptops`
  (returns (ReturnValue :type Boolean))
  (bind _newparam (`self.GetTopDownGame`))
  (return (< (`/Game/Base/BP_TopDownGameMode.nrLaptops` _newparam) (`/Game/Base/BP_TopDownGameMode.maxLaptops` _newparam))))

(fn `Check Nr Phones`
  (returns (ReturnValue :type Boolean))
  (bind _newparam (`self.GetTopDownGame`))
  (return (< (`/Game/Base/BP_TopDownGameMode.nrPhones` _newparam) (`/Game/Base/BP_TopDownGameMode.maxPhones` _newparam))))

(fn `Check Nr Tvs`
  (returns (ReturnValue :type Boolean))
  (bind _newparam (`self.GetTopDownGame`))
  (return (< (`/Game/Base/BP_TopDownGameMode.NrTvs` _newparam) (`/Game/Base/BP_TopDownGameMode.maxTVs` _newparam))))

(fn `CheckProgressBar`
  (if (>= (`self.progressSearching`) (`self.maxValueSearching`))
    (`self.DropItem`)
    (`self.K2_DestroyActor`)))

(fn `DropItem`
  (switch `int` (`KismetMathLibrary.RandomInteger` 13) :!label _label
    (:`0`
      (bind _returnvalue (`self.Check Nr Energy Drinks` :!label _label_2))
      (if _returnvalue
        (`self.Spawn Energy Drink`)
        (else
          (goto _label))))
    (:`1`
      (goto _label_2))
    (:`2`
      (goto _label_2))
    (:`3`
      (goto _label_2))
    (:`4`
      (bind _returnvalue_2 (`self.Check Nr Tvs`))
      (if _returnvalue_2
        (`self.Spawn TV`)
        (else
          (goto _label))))
    (:`5`
      (bind _returnvalue_3 (`self.Check Nr Balls` :!label _label_3))
      (if _returnvalue_3
        (`self.Spawn Ball`)
        (`KismetSystemLibrary.PrintString` "Ball")
        (else
          (goto _label))))
    (:`6`
      (goto _label_3))
    (:`7`
      (goto _label_3))
    (:`8`
      (bind _returnvalue_4 (`self.Check Nr Lamps` :!label _label_4))
      (if _returnvalue_4
        (`self.spawnLamp`)
        (else
          (goto _label))))
    (:`9`
      (goto _label_4))
    (:`10`
      (bind _returnvalue_5 (`self.Check Nr Phones` :!label _label_5))
      (if _returnvalue_5
        (`self.spawnPhone`)
        (else
          (goto _label))))
    (:`11`
      (goto _label_5))
    (:`12`
      (bind _returnvalue_6 (`self.Check Nr Laptops`))
      (if _returnvalue_6
        (`self.SpawnLaptop`)
        (else
          (goto _label))))))

(fn `GetTopDownGame`
  (returns (NewParam :type "/Game/Base/BP_TopDownGameMode Object Reference"))
  (bind _asbp_top_down_game_mode (cast `/Game/Base/BP_TopDownGameMode` (`GameplayStatics.GetGameMode`)))
  (return _asbp_top_down_game_mode))

(fn `Hide/ShowBar`
  (bind _widget (`self.Widget`))
  (bind _widget_2 (`self.Widget`))
  ;[1 1 1] Hide / Show to progress bar UI when searching object or not
  (bind _newparam (`self.CheckRunningState`))
  (if _newparam
    (`SceneComponent.SetVisibility` _widget_2 false false :!label _label) ; Hide Bar
    (elif (`self.PickingUpItem`)
      (if (`KismetSystemLibrary.IsValid` _widget)
        (`SceneComponent.SetVisibility` _widget true false) ; Show Bar
      )
      (elif (`KismetSystemLibrary.IsValid` _widget_2)
        (goto _label)))))

(fn `PickingUpAnimation`
  (`SceneComponent.K2_AddRelativeLocation` (`self.VisualMesh`) (`KismetMathLibrary.MakeVector` 0.0 0.0 (* (`KismetMathLibrary.Sin` (* (`self.GetGameTimeSinceCreation`) 20.0)) 5.0)) false false))

(fn `SearchForItem`
  ;[1 1 1] Progress of searching an item in the box.
  (if (`self.PickingUpItem`)
    (if (<= (`self.progressSearching`) (`self.maxValueSearching`))
      (set `self.progressSearching` (+ (* (`GameplayStatics.GetWorldDeltaSeconds`) (`self.progressSearchInc`)) (`self.progressSearching`))))))

(fn `Spawn Ball`
  (`|SpawnActorFromClass` "/Game/Code/Items/BP_Ball.BP_Ball_C" (`KismetMathLibrary.MakeTransform` (`SceneComponent.K2_GetComponentLocation` (`self.SpawnPos`))) "Undefined" "OverrideRootScale" null null)
  (bind _newparam (`self.GetTopDownGame`))
  (set `/Game/Base/BP_TopDownGameMode.nrBalls` (+ (`/Game/Base/BP_TopDownGameMode.nrBalls` _newparam) 1) _newparam))

(fn `Spawn Energy Drink`
  (`|SpawnActorFromClass` "/Game/Code/Items/BP_EnergyDrink.BP_EnergyDrink_C" (`KismetMathLibrary.MakeTransform` (`SceneComponent.K2_GetComponentLocation` (`self.SpawnPos`))) "Undefined" "OverrideRootScale" null null)
  (bind _newparam (`self.GetTopDownGame`))
  (set `/Game/Base/BP_TopDownGameMode.NrEnergyDrinks` (+ (`/Game/Base/BP_TopDownGameMode.NrEnergyDrinks` _newparam) 1) _newparam))

(fn `Spawn TV`
  (`|SpawnActorFromClass` "/Game/Code/Items/BP_TV.BP_TV_C" (`KismetMathLibrary.MakeTransform` (`SceneComponent.K2_GetComponentLocation` (`self.SpawnPos`))) "Undefined" "OverrideRootScale" null null)
  (bind _newparam (`self.GetTopDownGame`))
  (set `/Game/Base/BP_TopDownGameMode.NrTvs` (+ (`/Game/Base/BP_TopDownGameMode.NrTvs` _newparam) 1) _newparam))

(fn `spawnLamp`
  (`|SpawnActorFromClass` "/Game/Code/Items/BP_Lamp.BP_Lamp_C" (`KismetMathLibrary.MakeTransform` (`SceneComponent.K2_GetComponentLocation` (`self.SpawnPos`))) "Undefined" "OverrideRootScale" null null)
  (bind _newparam (`self.GetTopDownGame`))
  (set `/Game/Base/BP_TopDownGameMode.nrLamps` (+ (`/Game/Base/BP_TopDownGameMode.nrLamps` _newparam) 1) _newparam)
  (`KismetSystemLibrary.PrintString` "Lamp"))

(fn `SpawnLaptop`
  (`|SpawnActorFromClass` "/Game/Code/Items/BP_Laptop.BP_Laptop_C" (`KismetMathLibrary.MakeTransform` (`SceneComponent.K2_GetComponentLocation` (`self.SpawnPos`))) "Undefined" "OverrideRootScale" null null)
  (bind _newparam (`self.GetTopDownGame`))
  (set `/Game/Base/BP_TopDownGameMode.nrLaptops` (+ (`/Game/Base/BP_TopDownGameMode.nrLaptops` _newparam) 1) _newparam))

(fn `spawnPhone`
  (`|SpawnActorFromClass` "/Game/Code/Items/BP_Phone.BP_Phone_C" (`KismetMathLibrary.MakeTransform` (`SceneComponent.K2_GetComponentLocation` (`self.SpawnPos`))) "Undefined" "OverrideRootScale" null null)
  (bind _newparam (`self.GetTopDownGame`))
  (set `/Game/Base/BP_TopDownGameMode.nrPhones` (+ (`/Game/Base/BP_TopDownGameMode.nrPhones` _newparam) 1) _newparam))

(fn `UpdateUIBar`
  ;[1 1 1] Update the UI of the Progress Bar for the RandomItem Actor
  (bind _aswbp_progress_bar (cast `/Game/Code/UI/WBP_ProgressBar` (`WidgetComponent.GetUserWidgetObject` (`self.Widget`))))
  (`ProgressBar.SetPercent` (`/Game/Code/UI/WBP_ProgressBar.ProgressBar_0` _aswbp_progress_bar) (/ (`self.progressSearching`) (`self.maxValueSearching`))) ; Set Bar %
)

(fn `UserConstructionScript`
  (`parent.UserConstructionScript`))