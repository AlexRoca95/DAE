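; BP_Truck is the player's drop-off point for stolen items and the escape point.
; On collision box overlap it enables input and, if the game mode is in its running state, triggers PlayerEscape.
; Otherwise, a player carrying stolen items gets the E key prompt and opens a Gate that lets the Drop item input call DropAllObjects.
; Leaving the box hides the prompt and closes the Gate.
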(event `InputAction|Drop item`
  (params (Key :type "Key Structure"))
  (:`Pressed`
    (`/Engine/EditorBlueprintResources/StandardMacros.Gate` true :!label _label
      (:`Exit`
        (set `/Game/Code/Characters/BP_Player.firstShowedE` false (stale `self.CollisionBox.OnComponentBeginOverlap` _asbp_player))
        (`/Game/Code/Characters/BP_Player.DropAllObjects` (stale `self.CollisionBox.OnComponentBeginOverlap` _asbp_player))))))

(event `self.CollisionBox.OnComponentBeginOverlap`
  (params (OverlappedComponent :type "PrimitiveComponent Object Reference") (OtherActor :type "Actor Object Reference") (OtherComp :type "PrimitiveComponent Object Reference") (OtherBodyIndex :type Integer) (bFromSweep :type Boolean) (SweepResult :type "HitResult Structure (by ref)"))
  (bind _asbp_player (cast `/Game/Code/Characters/BP_Player` OtherActor))
  (`self.EnableInput` (`GameplayStatics.GetPlayerController` 0))
  (bind _asbp_top_down_game_mode (cast `/Game/Base/BP_TopDownGameMode` (`GameplayStatics.GetGameMode`)))
  (if (`/Game/Base/BP_TopDownGameMode.isRunningState` _asbp_top_down_game_mode)
    (`/Game/Base/BP_TopDownGameMode.PlayerEscape` _asbp_top_down_game_mode)
    (else
      ;[1 1 1] Check if player carrying objects to drop
      (if (> (`KismetArrayLibrary.Array_Length` (`/Game/Code/Characters/BP_Player.stolenItems` _asbp_player)) 0)
        (set `/Game/Code/Characters/BP_Player.showEKey` true _asbp_player)
        (goto _label :!via `Open`)))))

(event `self.CollisionBox.OnComponentEndOverlap`
  (params (OverlappedComponent :type "PrimitiveComponent Object Reference") (OtherActor :type "Actor Object Reference") (OtherComp :type "PrimitiveComponent Object Reference") (OtherBodyIndex :type Integer))
  (bind _asbp_player (cast `/Game/Code/Characters/BP_Player` OtherActor))
  (set `/Game/Code/Characters/BP_Player.showEKey` false _asbp_player)
  (goto _label :!via `Close`))

(fn `UserConstructionScript`
  (`parent.UserConstructionScript`))