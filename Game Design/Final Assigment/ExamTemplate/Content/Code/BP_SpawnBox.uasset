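; BP_SpawnBox is a spawn point that randomly places a BP_RandomItem at its SpawnPos location.
; On BeginPlay it makes a random-bool spawn attempt, setting ItemSpawned and incrementing BP_TopDownGameMode's NrItems on success.
; While empty, it retries every Tick as long as NrItems is below MinItems.
; The TotalItems cap limits only the counter increment, not the spawn itself.
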(event `self.ReceiveBeginPlay`
  (`parent.ReceiveBeginPlay`)
  (`self.SpawnItem`))

(event `self.ReceiveTick`
  (params (DeltaSeconds :type "Float (single-precision)"))
  (`parent.ReceiveTick` DeltaSeconds)
  (`self.CheckNrItems`))

(fn `CheckNrItems`
  ;[1 1 1] Check if we have reached the min Items to spawn and spawn one if not.
  (if (not (`self.ItemSpawned`))
    (bind _asbp_top_down_game_mode (cast `/Game/Base/BP_TopDownGameMode` (`GameplayStatics.GetGameMode`)))
    (bind _newparam (`/Game/Base/BP_TopDownGameMode.GetNrItems` _asbp_top_down_game_mode))
    (bind _newparam_2 (`/Game/Base/BP_TopDownGameMode.GetMinItems` _asbp_top_down_game_mode))
    (if (< _newparam _newparam_2)
      (`self.SpawnItem`) ; Still need items to spawn
    )))

(fn `IncNrItems`
  ;[1 1 1] Increment the Nr of Items if we haven't reach the maximum value
  (bind _asbp_top_down_game_mode (cast `/Game/Base/BP_TopDownGameMode` (`GameplayStatics.GetGameMode`)))
  (bind _newparam (`/Game/Base/BP_TopDownGameMode.GetNrItems` _asbp_top_down_game_mode))
  (bind _newparam_2 (`/Game/Base/BP_TopDownGameMode.GetTotalItems` _asbp_top_down_game_mode))
  (if (< _newparam _newparam_2)
    (set `/Game/Base/BP_TopDownGameMode.NrItems` (+ _newparam 1.0) _asbp_top_down_game_mode)))

(fn `SpawnItem`
  (bind _returnvalue_location (`KismetMathLibrary.BreakTransform` (`SceneComponent.K2_GetComponentToWorld` (`self.SpawnPos`))))
  ;[1 1 1] Spawn an Item at the position if the SpawnBox Class (only if the random bool returned true)
  (if (`KismetMathLibrary.RandomBool`)
    (`self.IncNrItems`)
    (`|SpawnActorFromClass` "/Game/Code/BP_RandomItem.BP_RandomItem_C" (`KismetMathLibrary.MakeTransform` _returnvalue_location) "Undefined" "OverrideRootScale" null null)
    (set `self.ItemSpawned` true) ; This Spawn box has an Item
  ))

(fn `UserConstructionScript`
  (`parent.UserConstructionScript`))