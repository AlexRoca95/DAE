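; BP_SpawnBackpack is a spawn point that randomly spawns a BP_Backpack at its SpawnPos component.
; On BeginPlay and every Tick it checks the BackpackSpawned flag on BP_TopDownGameMode and, while that is false, calls SpawnBackPack.
; SpawnBackPack makes a random bool roll and, on success, spawns the backpack and sets the shared flag, stopping further attempts by any instance.
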(event `self.ReceiveBeginPlay`
  (`parent.ReceiveBeginPlay`)
  (bind _asbp_top_down_game_mode (cast `/Game/Base/BP_TopDownGameMode` (`GameplayStatics.GetGameMode`)))
  (if (not (`/Game/Base/BP_TopDownGameMode.BackpackSpawned` _asbp_top_down_game_mode))
    (`self.spawnBackPack`)))

(event `self.ReceiveTick`
  (params (DeltaSeconds :type "Float (single-precision)"))
  (`parent.ReceiveTick` DeltaSeconds)
  (bind _asbp_top_down_game_mode (cast `/Game/Base/BP_TopDownGameMode` (`GameplayStatics.GetGameMode`)))
  (if (not (`/Game/Base/BP_TopDownGameMode.BackpackSpawned` _asbp_top_down_game_mode))
    (`self.spawnBackPack`)))

(fn `spawnBackPack`
  (if (`KismetMathLibrary.RandomBool`)
    (`|SpawnActorFromClass` "/Game/Code/Items/BP_Backpack.BP_Backpack_C" (`KismetMathLibrary.MakeTransform` (`SceneComponent.K2_GetComponentLocation` (`self.SpawnPos`))) "Undefined" "OverrideRootScale" null null)
    (bind _asbp_top_down_game_mode (cast `/Game/Base/BP_TopDownGameMode` (`GameplayStatics.GetGameMode`)))
    (set `/Game/Base/BP_TopDownGameMode.BackpackSpawned` true _asbp_top_down_game_mode)))

(fn `UserConstructionScript`
  (`parent.UserConstructionScript`))