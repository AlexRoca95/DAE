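; BP_Entrance is an entrance actor that lets the player drop all carried objects once they have overlapped it.
; Any overlap enables player 0's input on the actor, then a successful cast to BP_Player stores the player and opens a gate.
; The Drop item press passes through that gate to call DropAllObjects on the stored player.
; Nothing closes the gate or disables input when the overlap ends.
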(event `InputAction|Drop item`
  (params (Key :type "Key Structure"))
  (:`Pressed`
    (`/Engine/EditorBlueprintResources/StandardMacros.Gate` true :!label _label
      (:`Exit`
        (`/Game/Code/Characters/BP_Player.DropAllObjects` (stale `self.ReceiveActorBeginOverlap` _asbp_player))))))

(event `self.ReceiveActorBeginOverlap`
  (params (OtherActor :type "Actor Object Reference"))
  (`self.EnableInput` (`GameplayStatics.GetPlayerController` 0))
  (bind _asbp_player (cast `/Game/Code/Characters/BP_Player` OtherActor))
  (goto _label :!via `Open`))

(fn `UserConstructionScript`
  (`parent.UserConstructionScript`))