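; BP_Ball is a ball item that spins and floats in place, built on a parent Blueprint.
; On BeginPlay it runs the parent logic, then sets its size and price from ball-specific values, assigns its type enum and marks itself as not closed.
; Each Tick calls the parent, then Rotate and Floating to animate it.
; The overlap event and construction script add no logic of their own.
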(event `self.ReceiveBeginPlay`
  (`parent.ReceiveBeginPlay`)
  (`|ExecutionSequence`
    (:`then_0`
      (set `self.size` (`self.sizeBall`)))
    (:`then_1`
      (set `self.Price` (`self.BallPrice`)))
    (:`then_2`
      (set `self.type` "NewEnumerator8"))
    (:`then_3`
      (set `self.isClosed` false))))

(event `self.ReceiveActorBeginOverlap`
  (params (OtherActor :type "Actor Object Reference")))

(event `self.ReceiveTick`
  (params (DeltaSeconds :type "Float (single-precision)"))
  (`parent.ReceiveTick` DeltaSeconds)
  (`|ExecutionSequence`
    (:`then_0`
      (`self.rotate`))
    (:`then_1`
      (`self.floating`))))

(fn `UserConstructionScript`
  (`parent.UserConstructionScript`))