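; BP_Laptop is a laptop item Blueprint that rotates and floats in the world.
; On BeginPlay it calls its parent, then fills in Price and Size from laptop-specific values, sets its Type enum and marks IsClosed false.
; Every Tick calls the parent, then Rotate and Floating to animate the item.
; The construction script only calls the parent, and the overlap event is disabled.
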(event `self.ReceiveBeginPlay`
  (`parent.ReceiveBeginPlay`)
  (`|ExecutionSequence`
    (:`then_0`
      (set `self.Price` (`self.laptopPrice`)))
    (:`then_1`
      (set `self.size` (`self.laptopSize`)))
    (:`then_2`
      (set `self.type` "NewEnumerator9"))
    (:`then_3`
      (set `self.isClosed` false))))

(event `self.ReceiveTick`
  (params (DeltaSeconds :type "Float (single-precision)"))
  (`parent.ReceiveTick` DeltaSeconds)
  (`|ExecutionSequence`
    (:`then_0`
      (`self.rotate`))
    (:`then_1`
      (`self.floating`))))

(fn `UserConstructionScript`
  (`parent.UserConstructionScript`))