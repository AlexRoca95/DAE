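; BP_Phone is a phone pickup item that spins and floats in the world until the player collects it.
; On BeginPlay it sets its price and size from phone-specific values, and every Tick calls Rotate and Floating.
; Overlapping the pickup collision enables input, and a Gate opens only while BP_Player is inside, letting the Pick Up Item action call PickUpItem with the phone and its size.
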(event `self.ReceiveBeginPlay`
  (`parent.ReceiveBeginPlay`)
  (`|ExecutionSequence`
    (:`then_0`
      (set `self.Price` (`self.phonePrice`)))
    (:`then_1`
      (set `self.size` (`self.phoneSize`)))))

(event `self.ReceiveTick`
  (params (DeltaSeconds :type "Float (single-precision)"))
  (`parent.ReceiveTick` DeltaSeconds)
  (`|ExecutionSequence`
    (:`then_0`
      (`self.rotate`))
    (:`then_1`
      (`self.floating`))))

(event `InputAction|Pick Up Item`
  (params (Key :type "Key Structure"))
  ;[1 1 1] Pick Up Item
  (:`Pressed`
    (`/Engine/EditorBlueprintResources/StandardMacros.Gate` false :!label _label
      (:`Exit`
        (`self.PickUpItem` "BP_Phone_C" (`self.phoneSize`))))))

(event `self.PickUpCollision.OnComponentBeginOverlap`
  (params (OverlappedComponent :type "PrimitiveComponent Object Reference") (OtherActor :type "Actor Object Reference") (OtherComp :type "PrimitiveComponent Object Reference") (OtherBodyIndex :type Integer) (bFromSweep :type Boolean) (SweepResult :type "HitResult Structure (by ref)"))
  ;[1 1 1] Pick Up Item
  (`self.EnableInput` (`GameplayStatics.GetPlayerController` 0))
  (cast `/Game/Code/Characters/BP_Player` OtherActor)
  (goto _label :!via `Open`))

(event `self.PickUpCollision.OnComponentEndOverlap`
  (params (OverlappedComponent :type "PrimitiveComponent Object Reference") (OtherActor :type "Actor Object Reference") (OtherComp :type "PrimitiveComponent Object Reference") (OtherBodyIndex :type Integer))
  ;[1 1 1] Pick Up Item
  (cast `/Game/Code/Characters/BP_Player` OtherActor)
  (goto _label :!via `Close`))

(fn `UserConstructionScript`
  (`parent.UserConstructionScript`))