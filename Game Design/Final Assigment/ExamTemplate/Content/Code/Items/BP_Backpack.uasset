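; BP_Backpack is a pickup item that expands the player's inventory space.
; Overlap on PickUpCollision enables input and, for a BP_Player, opens a Gate that closes again when the player leaves.
; Pressing Pick Up Item through the open Gate calls PickUpBackpack, which adds BagSpace to the player's MaxSpace and SpaceLeft and sets HaveBackpack.
; The backpack actor then destroys itself.
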(event `InputAction|Pick Up Item`
  (params (Key :type "Key Structure"))
  (:`Pressed`
    (`/Engine/EditorBlueprintResources/StandardMacros.Gate` false :!label _label
      (:`Exit`
        (`self.PickUpBackpack`)
        (`self.K2_DestroyActor`)))))

(event `self.PickUp collision.OnComponentBeginOverlap`
  (params (OverlappedComponent :type "PrimitiveComponent Object Reference") (OtherActor :type "Actor Object Reference") (OtherComp :type "PrimitiveComponent Object Reference") (OtherBodyIndex :type Integer) (bFromSweep :type Boolean) (SweepResult :type "HitResult Structure (by ref)"))
  (`self.EnableInput` (`GameplayStatics.GetPlayerController` 0))
  (cast `/Game/Code/Characters/BP_Player` OtherActor)
  (goto _label :!via `Open`))

(event `self.PickUp collision.OnComponentEndOverlap`
  (params (OverlappedComponent :type "PrimitiveComponent Object Reference") (OtherActor :type "Actor Object Reference") (OtherComp :type "PrimitiveComponent Object Reference") (OtherBodyIndex :type Integer))
  (cast `/Game/Code/Characters/BP_Player` OtherActor)
  (goto _label :!via `Close`))

(fn `PickUpBackpack`
  (bind _bagspace (`self.bagSpace`))
  ;[1 1 1] Increment the max space for the player
  (bind _asbp_player (cast `/Game/Code/Characters/BP_Player` (`GameplayStatics.GetPlayerCharacter` 0)))
  (set `/Game/Code/Characters/BP_Player.maxSpace` (+ (`/Game/Code/Characters/BP_Player.maxSpace` _asbp_player) _bagspace) _asbp_player)
  (set `/Game/Code/Characters/BP_Player.spaceLeft` (+ _bagspace (`/Game/Code/Characters/BP_Player.spaceLeft` _asbp_player)) _asbp_player)
  (set `/Game/Code/Characters/BP_Player.haveBackpack` true _asbp_player))

(fn `UserConstructionScript`
  (`parent.UserConstructionScript`))