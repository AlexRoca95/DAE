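; Hiding spot actor that lets the player hide by toggling the character's IsHiding flag and in-game visibility through UseHidingSpot.
; Tick polls that global player flag, swapping closed and open door components to match, regardless of which spot is used.
; Tick also bobs a Billboard marker on a sine of game time, and hides it once the player hides, with no code showing it again.
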(event `self.ReceiveBeginPlay`
  (`parent.ReceiveBeginPlay`)
  (`|ExecutionSequence`
    (:`then_0`
      (set `self.type` "NewEnumerator6"))
    (:`then_1`
      (set `self.isClosed` true))))

(event `self.ReceiveTick`
  (params (DeltaSeconds :type "Float (single-precision)"))
  (`parent.ReceiveTick` DeltaSeconds)
  (`|ExecutionSequence`
    (:`then_0`
      (bind _asbp_player (cast `/Game/Code/Characters/BP_Player` (`GameplayStatics.GetPlayerCharacter` 0)))
      (if (`/Game/Code/Characters/BP_Player.isHiding` _asbp_player)
        (`self.Close Hiding Spot`)
        (`SceneComponent.SetVisibility` (`self.Billboard`) false false)
        (else
          (`self.Open Hiding Spot`))))
    (:`then_1`
      (`SceneComponent.K2_AddRelativeLocation` (`self.Billboard`) (`KismetMathLibrary.MakeVector` 0.0 0.0 (* (`KismetMathLibrary.Sin` (`self.GetGameTimeSinceCreation`)) 1.0)) false false))))

(fn `Close Hiding Spot`
  (`|ExecutionSequence`
    (:`then_0`
      (`SceneComponent.SetVisibility` (`self.Door closed`) true false))
    (:`then_1`
      (`SceneComponent.SetVisibility` (`self.Door open`) false false))))

(fn `Open Hiding Spot`
  (`|ExecutionSequence`
    (:`then_0`
      (`SceneComponent.SetVisibility` (`self.Door closed`) false false))
    (:`then_1`
      (`SceneComponent.SetVisibility` (`self.Door open`) true false))))

(fn `Use Hiding Spot`
  (bind _asbp_player (cast `/Game/Code/Characters/BP_Player` (`GameplayStatics.GetPlayerCharacter` 0)))
  (if (`/Game/Code/Characters/BP_Player.isHiding` _asbp_player)
    (`self.SetActorHiddenInGame` _asbp_player false)
    (set `/Game/Code/Characters/BP_Player.isHiding` false _asbp_player)
    (else
      (`self.SetActorHiddenInGame` _asbp_player true)
      (set `/Game/Code/Characters/BP_Player.isHiding` true _asbp_player))))

(fn `UserConstructionScript`
  (`parent.UserConstructionScript`))