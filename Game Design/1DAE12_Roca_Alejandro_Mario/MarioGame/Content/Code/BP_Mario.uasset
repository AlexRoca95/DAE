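; BP_Mario is the player character, moved along the Y axis by input, with a spotlight that shrinks over time.
; Movement offsets the location without sweep or delta-time scaling, while Jump adds a capsule impulse when a downward sphere trace hits.
; Tick narrows the spotlight cone and flags LightOff near zero; overlapping a BP_Torch resets both.
; Destroying the actor reloads the current level.
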(event `self.ReceiveActorBeginOverlap`
  (params (OtherActor :type "Actor Object Reference"))
  (cast `/Game/Code/BP_Torch` OtherActor)
  (set `self.LightRadius` 10.0) ; Torch pick up reset torch light timer
  (set `self.LightOff` false))

(event `self.ReceiveTick`
  (params (DeltaSeconds :type "Float (single-precision)"))
  (`self.UpdateLightRadius` DeltaSeconds))

(event `self.ReceiveDestroyed`
  (bind _returnvalue (`GameplayStatics.GetCurrentLevelName` true))
  (`GameplayStatics.OpenLevel` (`KismetStringLibrary.Conv_StringToName` _returnvalue)))

(event `InputAction|Jump`
  (params (Key :type "Key Structure"))
  (:`Pressed`
    (`self.Jumping`)))

(event `InputAxis|MoveRight`
  (params (AxisValue :type "Float (single-precision)"))
  (`self.Movement` AxisValue))

(fn `Jumping`
  (bind _returnvalue (`self.K2_GetActorLocation`))
  (bind _capsule (`self.Capsule`))
  (bind (_outhit _returnvalue_2) (`KismetSystemLibrary.SphereTraceSingle` :`Start` _returnvalue :`End` (- _returnvalue (`KismetMathLibrary.MakeVector` 0.0 0.0 (`CapsuleComponent.CapsuleHalfHeight` _capsule))) :`Radius` (`CapsuleComponent.CapsuleRadius` _capsule) :`TraceChannel` "TraceTypeQuery1" :`DrawDebugType` "ForDuration")) ; Collision Test
  (if _returnvalue_2
    (`PrimitiveComponent.AddImpulse` (`self.Capsule`) (`KismetMathLibrary.MakeVector` 0.0 0.0 (`self.JumpForce`)) "None" true) ; Only if Collide with ground
    (`KismetSystemLibrary.PrintString` "Jump")))

(fn `Movement`
  (params (B :type "Float (double-precision)"))
  (`self.K2_SetActorLocation` (+ (`self.K2_GetActorLocation`) (* (`KismetMathLibrary.MakeVector` 0.0 (`self.WalkSpeed`)) B))) ; Set Mario Position
)

(fn `UpdateLightRadius`
  (params (B :type "Float (double-precision)"))
  (bind _output_get (set `self.LightRadius` (- (`self.LightRadius`) B)))
  (`SpotLightComponent.SetOuterConeAngle` (`self.SpotLight`) _output_get) ; Change radius light
  (if (< (`self.LightRadius`) 0.5)
    (set `self.LightOff` true)
    (`KismetSystemLibrary.PrintString` "light off")))

(fn `UserConstructionScript`)