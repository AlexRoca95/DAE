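; BP_Block is a Mario-style item block that releases a mushroom once when BP_Mario hits it.
; An overlap on HitSpot raises BlockPickUp with MoveComponentTo and spawns BP_Mushrom at SpawnPos.
; It then destroys HitSpot so the block cannot trigger again, and after a short delay lowers BlockPickUp back to complete the bump.
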(event `self.HitSpot.OnComponentBeginOverlap`
  (params (OverlappedComponent :type "PrimitiveComponent Object Reference") (OtherActor :type "Actor Object Reference") (OtherComp :type "PrimitiveComponent Object Reference") (OtherBodyIndex :type Integer) (bFromSweep :type Boolean) (SweepResult :type "HitResult Structure (by ref)"))
  (bind _blockpickup (`self.BlockPickUp`))
  (bind _blockpickup_2 (`self.BlockPickUp`))
  (bind (_returnvalue_location _returnvalue_rotation) (`KismetMathLibrary.BreakTransform` (`SceneComponent.GetRelativeTransform` _blockpickup)))
  (bind (_returnvalue_location_2 _returnvalue_rotation_2) (`KismetMathLibrary.BreakTransform` (`SceneComponent.GetRelativeTransform` _blockpickup_2)))
  (cast `/Game/Code/BP_Mario` OtherActor)
  (`KismetSystemLibrary.MoveComponentTo` _blockpickup_2 (+ _returnvalue_location_2 (0.0 0.0 30.0)) _returnvalue_rotation_2) ; Moves up
  (`|SpawnActorFromClass` "/Game/Code/BP_Mushrom.BP_Mushrom_C" (`SceneComponent.K2_GetComponentToWorld` (`self.SpawnPos`)) "Undefined" "OverrideRootScale" null null)
  (`ActorComponent.K2_DestroyComponent` (`self.HitSpot`)) ; Cannot collide anymore
  (`KismetSystemLibrary.Delay` 0.3)
  (`KismetSystemLibrary.MoveComponentTo` _blockpickup (+ _returnvalue_location (0.0 0.0 -30.0)) _returnvalue_rotation) ; Back origin pos
)

(fn `UserConstructionScript`)